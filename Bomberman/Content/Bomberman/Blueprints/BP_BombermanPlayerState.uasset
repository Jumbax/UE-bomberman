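; BP_BombermanPlayerState is the Bomberman player state Blueprint that keeps a minutes-and-seconds countdown.
; StartTimer sets a looping one-second timer that fires SetTimer.
; Each tick decrements Seconds, or at zero decrements Minutes and resets Seconds to 59.
; The graph has no check for the countdown reaching zero and never clears the timer.
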(event Custom|SetTimer
  (if (> (Variables|Default|GetSeconds) 0)
    (bind _result (Math|Integer|DecrementInt (Variables|Default|GetSeconds))
      (:%20%20
        (Variables|Default|SetSeconds _result)))
    (elif (== (Variables|Default|GetSeconds) 0)
      (bind _result_2 (Math|Integer|DecrementInt (Variables|Default|GetMinutes))
        (:%20%20
          (Variables|Default|SetMinutes _result_2)
          (Variables|Default|SetSeconds 59))))))

(event Custom|StartTimer
  (Utilities|Time|SetTimerbyEvent (delegate Custom|SetTimer) 1.0 true))

(fn ConstructionScript)