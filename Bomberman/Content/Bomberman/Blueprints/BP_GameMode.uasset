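; Game mode for a Bomberman game that spawns players as they log in and starts the match once the lobby is full.
; Each login spawns and possesses a BP_BombermanPlayer at the first entry in SpawnLocations, then removes that entry so each spot is used once.
; When the player count reaches PlayersNumber, it sets GameStarted on every controller and starts each player state's timer.
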(event EventPostLogin
  (params (NewPlayer :type Player%20Controller%20Object%20Reference))
  (bind _returnvalue (Game|SpawnActorfromClass "/Game/Bomberman/Blueprints/BP_BombermanPlayer.BP_BombermanPlayer_C" (Math|Transform|MakeTransform (Utilities|Array|Get(acopy) (Variables|Default|GetSpawnLocations))) "AlwaysSpawn" 0 0))
  (Pawn|Possess NewPlayer _returnvalue)
  (Utilities|Array|RemoveIndex (Variables|Default|GetSpawnLocations))
  (Utilities|Array|Add (Variables|Default|GetPlayers) NewPlayer)
  (if (== (Utilities|Array|Length (Variables|Default|GetPlayers)) (Variables|Default|GetPlayersNumber))
    (for _array_element (Variables|Default|GetPlayers)
      (bind _asbp_bomberman_controller (Utilities|Casting|CastToBP_BombermanController _array_element))
      (Variables|/Game/Bomberman/Blueprints/BP_BombermanController.BP_BombermanController_C|SetGameStarted _asbp_bomberman_controller true)
      (bind _asbp_bomberman_player_state (Utilities|Casting|CastToBP_BombermanPlayerState (Variables|/Script/Engine.Controller|GetPlayerState _asbp_bomberman_controller)))
      (Default|StartTimer _asbp_bomberman_player_state))))

(fn ConstructionScript)